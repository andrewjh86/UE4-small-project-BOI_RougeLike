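; Actor component that drifts a BP_CloudMask_Object owner through the world to move its cloud mask.
; On BeginPlay it casts and caches the owner, then starts a looping timer at the PushRepetation interval.
; Each timer call teleports the owner by the world-space PushAmount offset, with rotation set to zero, then calls UpdateMaskGenerator on it.
; Movement is stepped by the timer, with Tick unused.
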(event Custom|CloudPush
  (bind _owneractor (Variables|Default|GetOwnerActor))
  (Transformation|Teleport _owneractor (+ (Transformation|GetActorLocation _owneractor) (Variables|Default|GetPushAmount)) "0, 0, 0")
  (Default|UpdateMaskGenerator _owneractor))

(event EventBeginPlay
  (bind _asbp_cloud_mask_object (Utilities|Casting|CastToBP_CloudMask_Object (Components|GetOwner)))
  (Variables|Default|SetOwnerActor _asbp_cloud_mask_object)
  (Utilities|Time|SetTimerbyEvent (delegate Custom|CloudPush) (Variables|Default|GetPushRepetation) true))

(event EventTick
  (params (DeltaSeconds :type Float%20%28single-precision%29)))